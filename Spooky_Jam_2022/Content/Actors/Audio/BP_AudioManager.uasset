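; Audio manager that plays cue-driven dialogue, prop sounds and footsteps, scaling them with round progress read from the Cat_Painting.
; TriggerSound routes each cue to dialogue sets, a per-object prop library, footsteps or death lines, which block later dialogue.
; Intensity, the elapsed fraction of the round, plus random jitter picks the index within most sound arrays.
; Tick also adjusts OOOO, rain and fireplace ambience volumes over the round.
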(event `self.ReceiveBeginPlay`
  (bind _audiocomponent (`AmbientSound.AudioComponent` (`self.OOOO`)))
  (set `self.Player` (cast `/Game/Actors/FP_Character` (`GameplayStatics.GetPlayerCharacter` 0) :!pure true))
  (bind _returnvalue (`GameplayStatics.GetActorOfClass` "/Game/Actors/Cat_Painting.Cat_Painting_C"))
  (set `self.Painting` _returnvalue)
  (`AudioComponent.SetPitchMultiplier` _audiocomponent (+ (`AudioComponent.PitchMultiplier` _audiocomponent) (`KismetMathLibrary.RandomFloatInRange` -0.1 0.05))))

(event `AudioTest`
  ;[0 0 0] Debug
  (`self.TriggerSound` "NewEnumerator2")
  (`KismetSystemLibrary.PrintString` "Hello"))

(event `self.ReceiveTick`
  (params (DeltaSeconds :type "Float (single-precision)"))
  (bind _painting (`self.Painting`))
  (bind _roundduration (`/Game/Actors/Cat_Painting.roundDuration` _painting))
  (bind _returnvalue (- (`GameplayStatics.GetTimeSeconds`) (`/Game/Actors/Cat_Painting.startTime` _painting)))
  (`AudioComponent.SetVolumeMultiplier` (`AmbientSound.AudioComponent` (`self.OOOO`)) (`KismetMathLibrary.MapRangeClamped` (- _returnvalue 30.0) 0.0 (- _roundduration 30.0) 0.0 0.25))
  (`AudioComponent.SetVolumeMultiplier` (`AmbientSound.AudioComponent` (`self.Rain`)) (`KismetMathLibrary.MapRangeClamped` _returnvalue 0.0 _roundduration 0.2 0.4))
  (`AudioComponent.SetVolumeMultiplier` (`AmbientSound.AudioComponent` (`self.Fireplace`)) (`KismetMathLibrary.MapRangeClamped` _returnvalue 0.0 _roundduration 0.2 0.4)))

(fn `Play Dialogue Interrupting`
  (params (Dialogue :type "DialogueWave Object Reference"))
  (bind _returnvalue (`GameplayStatics.GetPlayerCharacter` 0))
  (if (not (`self.Dead`))
    (bind _dialogue (`self.Dialogue`)
      (:`then`
        (`AudioComponent.Stop` _dialogue))
      (:`else`
        _))
    (bind _returnvalue_2 (`GameplayStatics.SpawnDialogueAttached` Dialogue (make `DialogueContext` "/Game/Audio/DialogueVoice.DialogueVoice" (`|MakeArray` "/Game/Audio/DialogueVoice.DialogueVoice" :!type "DialogueVoice Object Reference")) (`Actor.RootComponent` (cast `/Game/Actors/FP_Character` _returnvalue :!pure true)) "None" (`self.K2_GetActorLocation` _returnvalue) (struct) "KeepRelativeOffset" false 1.0 1.0 0.0 null))
    (set `self.Dialogue` _returnvalue_2)))

(fn `SelectAudioByIntensity`
  (params (Intensity :type "Float (double-precision)") (LastIndex :type Integer))
  (returns (SoundIndex :type Integer))
  (return (`KismetMathLibrary.Clamp` (`KismetMathLibrary.FFloor` (`KismetMathLibrary.MapRangeClamped` (+ Intensity (`KismetMathLibrary.MapRangeClamped` (`KismetMathLibrary.MultiplyMultiply_FloatFloat` (`KismetMathLibrary.RandomFloatInRange` -1.0 1.0) 1.8) -1.0 1.0 (* 0.3 -1.0) 0.3)) 0.0 1.0 0.0 (`KismetMathLibrary.Conv_IntToDouble` LastIndex))) 0 LastIndex)))

(fn `SelectFromDialogueSetByIntensity`
  (params (Intensity :type "Float (double-precision)") (DialogueSet :type "Array of /Game/Actors/Audio/SDialogueSet Structure"))
  (returns (Dialogue :type "DialogueWave Object Reference"))
  (bind (_objectcuetypeoptional _sounds) (break `/Game/Actors/Audio/SDialogueSet` (`|GetArrayItem` DialogueSet (`KismetMathLibrary.RandomInteger` (`KismetArrayLibrary.Array_Length` DialogueSet)))))
  (bind _soundindex (`self.SelectAudioByIntensity` Intensity (`KismetArrayLibrary.Array_LastIndex` _sounds)))
  (return (`|GetArrayItem` _sounds _soundindex)))

(fn `SelectFromSoundSetByInteract`
  (params (Intensity :type "Float (double-precision)") (InteractType :type "/Game/Actors/Audio/EAudioCueType Enum" :default "NewEnumerator0") (SoundSets :type "Array of /Game/Actors/Audio/SSoundSet Structure"))
  (returns (Sound :type "SoundWave Object Reference"))
  (for _array_element SoundSets
    (bind (_objectcuetypeoptional _sounds) (break `/Game/Actors/Audio/SSoundSet` _array_element))
    (if (and (> (`KismetArrayLibrary.Array_Length` _sounds) 0) (`|EnumEquality` _objectcuetypeoptional InteractType))
      (bind _soundindex (`self.SelectAudioByIntensity` (`local.Intensity`) (`KismetArrayLibrary.Array_LastIndex` _sounds)))
      (return (`|GetArrayItem` _sounds _soundindex)))))

(fn `TriggerSound`
  (params (Cue :type "/Game/Actors/Audio/EAudioCueType Enum" :default "NewEnumerator0") (ObjectType :type "/Game/Actors/Audio/EAudioPropType Enum" :default "NewEnumerator0") (Location :type "Vector Structure"))
  (locals (Intensity :type "Float (double-precision)"))
  (bind _painting (`self.Painting`))
  (bind (_objectcuetypeoptional _sounds) (break `/Game/Actors/Audio/SDialogueSet` (`self.Deaths`)))
  (bind (_objectcuetypeoptional_2 _sounds_2) (break `/Game/Actors/Audio/SSoundSet` (select `/Game/Actors/Audio/EAudioCueType` (`local.Cue`) :`NewEnumerator7` (`self.Footsteps`))))
  (`KismetSystemLibrary.PrintString` (`KismetStringLibrary.Concat_StrStr` "Audio cue: " (`|GetEnumeratorNameAsString` Cue) " Object: " (`|GetEnumeratorNameAsString` ObjectType)))
  (set `local.Intensity` (`KismetMathLibrary.SafeDivide` (- (`GameplayStatics.GetTimeSeconds`) (`/Game/Actors/Cat_Painting.startTime` _painting)) (`/Game/Actors/Cat_Painting.roundDuration` _painting)))
  (switch `/Game/Actors/Audio/EAudioCueType` Cue
    (:`NewEnumerator0`
      (bind _dialogue (`self.SelectFromDialogueSetByIntensity` (`local.Intensity`) (select `/Game/Actors/Audio/EAudioCueType` (`local.Cue`) :`NewEnumerator0` (`self.SecureSoundSets`) :`NewEnumerator1` (`self.SuccessSoundSets`) :`NewEnumerator2` (`self.FailSoundSets`)) :!label _label))
      (`self.Play Dialogue Interrupting` _dialogue))
    (:`NewEnumerator1`
      (goto _label))
    (:`NewEnumerator2`
      (goto _label))
    (:`NewEnumerator3`
      (bind _sound (`self.SelectFromSoundSetByInteract` (`local.Intensity`) (`local.Cue`) (`.SoundSets_6_F8A8E6E5498BA8C04FF21A888F7747C5` (break `/Game/Actors/Audio/SPropSoundLibrary` (`BlueprintMapLibrary.Map_Find` (`self.PropSoundLibrary`) (`local.ObjectType`)))) :!label _label_2))
      (`GameplayStatics.PlaySoundAtLocation` _sound (`local.Location`) (struct) 1.0 1.0 0.0 null null null))
    (:`NewEnumerator4`
      (goto _label_2))
    (:`NewEnumerator5`
      (goto _label_2))
    (:`NewEnumerator6`
      (goto _label_2))
    (:`NewEnumerator7`
      (bind _soundindex (`self.SelectAudioByIntensity` (`local.Intensity`) (`KismetArrayLibrary.Array_LastIndex` _sounds_2)))
      (`GameplayStatics.PlaySound2D` (`|GetArrayItem` _sounds_2 _soundindex) 1.0 1.0 0.0 null null))
    (:`NewEnumerator9`
      ;[0 0 0] Death
      (`self.Play Dialogue Interrupting` (`|GetArrayItem` _sounds (`KismetMathLibrary.RandomIntegerInRange` 0 (`KismetArrayLibrary.Array_LastIndex` _sounds))))
      (set `self.Dead` true))))

(fn `UserConstructionScript`)